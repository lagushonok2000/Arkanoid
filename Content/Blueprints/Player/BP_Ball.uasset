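; Physics-driven Arkanoid ball that trails the player paddle until launched, then bounces around at a fixed speed.
; Each tick it snaps velocity to the four diagonals via a 45-degree rotate-and-round, and scales ball and paddle speed with the GameMode's bonus wave.
; Hits push gameplay blocks with radial impulses or play a sound otherwise; destruction calls DecrimentScore and respawns the ball.
; The construction script tints the ball per level.
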(event Custom|LaunchBall
  (params (BallDirection :type Vector))
  ;[0.4196 0.6863 1] Launch ball event
  (Variables|BallDefaults|SetbIsBallActive true)
  (Physics|AddImpulse (Variables|Default|GetBall) BallDirection "None" true)
  (Components|Activation|Activate (Variables|Default|GetParticleTrace) false))

(event Custom|ClampVelocity
  (bind _returnvalue (Transformation|GetVelocity))
  (bind _returnvalue_2 (Math|Rotator|MakeRotator 0.0 0.0 45.0))
  (bind _ballspeed (Variables|BallDefaults|GetBallSpeed))
  (bind _returnvalue_3 (Math|Vector|ClampVectorSize _returnvalue _ballspeed _ballspeed))
  ;[0.4196 0.6863 1] Clamp ball velocity
  (Physics|SetPhysicsLinearVelocity (Variables|Default|GetBall) (* (Math|Vector|UnrotateVector (Math|Rotator|GetRotationXVector (Math|Rotator|MakeRotator 0.0 0.0 (|((round((A/B)))*B) (.yaw (Math|Rotator|MakeRotfromX (Math|Vector|RotateVector _returnvalue_3 _returnvalue_2))) 9e+01))) _returnvalue_2) (Math|Vector|VectorLength _returnvalue_3)) false "None"))

(event Custom|UpdateBallPosition
  ;[0.4196 0.6863 1] Attach the ball to player paddle when not in active game
  (if (not (Variables|BallDefaults|GetbIsBallActive))
    (Transformation|SetActorLocation (Math|Interpolation|VInterpTo (Transformation|GetWorldLocation (Variables|Default|GetBall)) (+ (Transformation|GetWorldLocation (Variables|/Game/Blueprints/Player/BP_Player.BP_Player_C|GetBallSpawnPoint (Variables|Default|GetPlayerReference))) "-10.000000,0.000000, 0") 0.5 0.2) false false)))

(event EventBeginPlay
  ;[1 0.1804 0.1804] Begin Play
  ;[0.8549 1 0.5451] Save player reference
  (bind _asbp_player (Utilities|Casting|CastToBP_Player (Pawn|GetControlledPawn (Game|GetPlayerController 0))))
  (Variables|Default|SetPlayerReference _asbp_player)
  ;[0.8549 1 0.5451] Save game mode reference
  (bind _asgm_arkanoid (Utilities|Casting|CastToGM_Arkanoid (Game|GetGameMode)))
  (Variables|Default|SetGameModeReference _asgm_arkanoid))

(event Collision|EventHit
  (params (MyComp :type Primitive%20Component%20Object%20Reference) (Other :type Actor%20Object%20Reference) (OtherComp :type Primitive%20Component%20Object%20Reference) (bSelfMoved :type Boolean) (HitLocation :type Vector :default "0, 0, 0") (HitNormal :type Vector :default "0, 0, 0") (NormalImpulse :type Vector :default "0, 0, 0") (Hit :type Hit%20Result%20Structure%20%28by%20ref%29))
  ;[0.4196 0.6863 1] Play SFX on ball hit
  (bind _asbp_gameplay_block (Utilities|Casting|CastToBP_GameplayBlock Other)
    (:then
      (Physics|AddRadialImpulse (Variables|/Game/Blueprints/Player/BP_GameplayBlock.BP_GameplayBlock_C|GetBlock_01 _asbp_gameplay_block) HitLocation 1e+02 5e+03 "RIF_Constant" false))
    (:CastFailed
      (Audio|Components|Audio|Play (Variables|Default|GetAudio) 0.0))))

(event EventTick
  (params (DeltaSeconds :type Float%20%28single-precision%29))
  (bind _playerreference (Variables|Default|GetPlayerReference))
  (bind _gamemodereference (Variables|Default|GetGameModeReference))
  (bind _bonuswaves (Variables|/Game/Blueprints/Game/GM_Arkanoid.GM_Arkanoid_C|GetBonusWaves _gamemodereference))
  ;[1 0.1804 0.1804] Event Tick
  (CallFunction|UpdateBallPosition)
  (CallFunction|ClampVelocity)
  ;[0.4196 0.6863 1] Handle ball and player paddle speed based on current wave level
  (if (>= _bonuswaves 5)
    (Variables|BallDefaults|SetBallSpeed 2.25e+03)
    (Variables|/Game/Blueprints/Player/BP_Player.BP_Player_C|SetSpeed _playerreference 9e+02)
    (else
      (switch int _bonuswaves
        (:1
          (Variables|BallDefaults|SetBallSpeed 1.25e+03)
          (Variables|/Game/Blueprints/Player/BP_Player.BP_Player_C|SetSpeed _playerreference 5e+02))
        (:2
          (Variables|BallDefaults|SetBallSpeed 1.5e+03)
          (Variables|/Game/Blueprints/Player/BP_Player.BP_Player_C|SetSpeed _playerreference 6e+02))
        (:3
          (Variables|BallDefaults|SetBallSpeed 1.75e+03)
          (Variables|/Game/Blueprints/Player/BP_Player.BP_Player_C|SetSpeed _playerreference 7e+02))
        (:4
          (Variables|BallDefaults|SetBallSpeed 2e+03)
          (Variables|/Game/Blueprints/Player/BP_Player.BP_Player_C|SetSpeed _playerreference 8e+02))))))

(event EventDestroyed
  ;[0.4196 0.6863 1] Handle lost ball
  (Default|DecrimentScore (Variables|Default|GetGameModeReference))
  (Default|SpawnBall (Variables|Default|GetPlayerReference))
  (Audio|PlaySound2D "/Game/Sounds/SFX/S_8Bit_UIButton.S_8Bit_UIButton" 5.0 1.0 0.0 0 0))

(fn ConstructionScript
  (bind _returnvalue (Game|GetCurrentLevelName true))
  (switch string _returnvalue
    (:GameplayGangam
      (bind _returnvalue_2 (Rendering|Material|CreateDynamicMaterialInstance (Variables|Default|GetBall) 0 "/Game/Materials/M_BaseColor.M_BaseColor" "None" :!class /Script/Engine.PrimitiveComponent))
      (bind _output_get (LocalVariables|SetMID _returnvalue_2))
      (Rendering|Material|SetVectorParameterValue _output_get "Color" "(R=0.647059,G=0.000000,B=0.000000,A=1.000000)" :!class /Script/Engine.MaterialInstanceDynamic))
    (:GamePlayShapeOfYou
      (bind _returnvalue_3 (Rendering|Material|CreateDynamicMaterialInstance (Variables|Default|GetBall) 0 "/Game/Materials/M_BaseColor.M_BaseColor" "None" :!class /Script/Engine.PrimitiveComponent))
      (bind _output_get_2 (LocalVariables|SetMID _returnvalue_3))
      (Rendering|Material|SetVectorParameterValue _output_get_2 "Color" "(R=1.000000,G=1.000000,B=1.000000,A=1.000000)" :!class /Script/Engine.MaterialInstanceDynamic))
    (:GameplayPowerRangers
      (bind _returnvalue_4 (Rendering|Material|CreateDynamicMaterialInstance (Variables|Default|GetBall) 0 "/Game/Materials/M_BaseColor.M_BaseColor" "None" :!class /Script/Engine.PrimitiveComponent))
      (bind _output_get_3 (LocalVariables|SetMID _returnvalue_4))
      (Rendering|Material|SetVectorParameterValue _output_get_3 "Color" "(R=0.104814,G=0.670000,B=0.000000,A=1.000000)" :!class /Script/Engine.MaterialInstanceDynamic))))